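; Player controller that handles character selection, pawn spawning and possession, and health display updates.
; On BeginPlay a client-prefixed event shows the character selection widget and creates the main widget without adding it to the viewport.
; Selection passes through a server-prefixed event to the GameMode as an interface-style spawn request.
; SpawnPlayer spawns and possesses the chosen class, while health updates pass through a client event to the main widget.
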(event Custom|CL_UpdateHealthValue
  (params (Percent :type Float%20%28single-precision%29) (EnemyName :type String))
  (Default|UpdateHealth (Variables|Default|GetWB_Main) Percent EnemyName))

(event Custom|CL_InitWidgets
  (bind _returnvalue (UserInterface|CreateWidget "/Game/Blueprints/UI/WB_CharacterSelection.WB_CharacterSelection_C"))
  (bind _output_get (Variables|Default|SetWB%20Character%20Selection _returnvalue))
  (UserInterface|Viewport|AddtoViewport _output_get 0)
  (bind _returnvalue_2 (UserInterface|CreateWidget "/Game/Blueprints/UI/WB_Main.WB_Main_C"))
  (Variables|Default|SetWB_Main _returnvalue_2))

(event Custom|SRV_SelectCharacter
  (params (Player :type Actor%20Class%20Reference) (SpawnLocation :type Vector))
  (bind _gamemode (Class|BPIGameMode|GetGameModeRef(Message) (Game|GetGameMode)))
  (Class|BPIGameMode|RequestSpawnPlayer(Message) _gamemode self Player SpawnLocation))

(event EventSelectCharacter
  (params (Player :type Actor%20Class%20Reference) (SpawnLocation :type Vector :default "0, 0, 0"))
  (CallFunction|SRVSelectCharacter Player SpawnLocation))

(event EventSpawnPlayer
  (params (Player :type Actor%20Class%20Reference) (SpawnTransform :type Transform))
  (bind _returnvalue (Game|SpawnActorfromClass Player SpawnTransform "AdjustIfPossibleButAlwaysSpawn" "MultiplyWithRoot" 0 0))
  (bind _player (Class|BPIPlayerBase|GetPlayerRef(Message) _returnvalue))
  (Pawn|Possess _player))

(event EventBeginPlay
  (CallFunction|InitializeWidgets))

(event EventInitializeWidgets
  (CallFunction|CLInitWidgets))

(event EventUpdateHealthValue
  (params (Percent :type Float%20%28double-precision%29) (EnemyName :type String))
  (CallFunction|CLUpdateHealthValue Percent EnemyName))

(fn ConstructionScript)

(fn GetPlayerControllerRef
  (return self))