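; TM_DragonRoad is a tilemap Blueprint for the Dragon Road area that pauses the player camera inside its left and right trigger boxes.
; Begin overlap on LeftBox or RightBox pauses the camera for actors tagged Player, and end overlap unpauses it.
; The checks run only on authority, reaching each player through GetPlayerRef and PausePlayerCamera message calls rather than casts.
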(event OnComponentBeginOverlap(LeftBox)
  (params (OverlappedComponent :type Primitive%20Component%20Object%20Reference) (OtherActor :type Actor%20Object%20Reference) (OtherComp :type Primitive%20Component%20Object%20Reference) (OtherBodyIndex :type Integer) (bFromSweep :type Boolean) (SweepResult :type Hit%20Result%20Structure%20%28by%20ref%29))
  (Networking|SwitchHasAuthority
    (:Authority
      (if (Actor|ActorHasTag OtherActor "Player")
        (bind _player (Class|BPIPlayerBase|GetPlayerRef(Message) OtherActor))
        (Class|BPIPlayerBase|PausePlayerCamera(Message) _player true)))))

(event OnComponentEndOverlap(LeftBox)
  (params (OverlappedComponent :type Primitive%20Component%20Object%20Reference) (OtherActor :type Actor%20Object%20Reference) (OtherComp :type Primitive%20Component%20Object%20Reference) (OtherBodyIndex :type Integer))
  (Networking|SwitchHasAuthority
    (:Authority
      (if (Actor|ActorHasTag OtherActor "Player")
        (bind _player (Class|BPIPlayerBase|GetPlayerRef(Message) OtherActor))
        (Class|BPIPlayerBase|PausePlayerCamera(Message) _player false)))))

(event OnComponentBeginOverlap(RightBox)
  (params (OverlappedComponent :type Primitive%20Component%20Object%20Reference) (OtherActor :type Actor%20Object%20Reference) (OtherComp :type Primitive%20Component%20Object%20Reference) (OtherBodyIndex :type Integer) (bFromSweep :type Boolean) (SweepResult :type Hit%20Result%20Structure%20%28by%20ref%29))
  (Networking|SwitchHasAuthority
    (:Authority
      (if (Actor|ActorHasTag OtherActor "Player")
        (bind _player (Class|BPIPlayerBase|GetPlayerRef(Message) OtherActor))
        (Class|BPIPlayerBase|PausePlayerCamera(Message) _player true)))))

(event OnComponentEndOverlap(RightBox)
  (params (OverlappedComponent :type Primitive%20Component%20Object%20Reference) (OtherActor :type Actor%20Object%20Reference) (OtherComp :type Primitive%20Component%20Object%20Reference) (OtherBodyIndex :type Integer))
  (Networking|SwitchHasAuthority
    (:Authority
      (if (Actor|ActorHasTag OtherActor "Player")
        (bind _player (Class|BPIPlayerBase|GetPlayerRef(Message) OtherActor))
        (Class|BPIPlayerBase|PausePlayerCamera(Message) _player false)))))

(fn ConstructionScript)