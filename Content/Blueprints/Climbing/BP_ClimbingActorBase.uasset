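; BP_ClimbingActorBase is a base actor for climbable objects, using two trigger volumes to tell players when and how they can climb.
; Box overlaps toggle the player's climb permission, passing this actor as the climbing object on entry and printing debug strings.
; UpperBox marks the upper limit, disabling upward climbing while overlapped and restoring it on exit.
; All overlaps run only on the server, filter by "Player" tag and notify through message calls.
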(event OnComponentBeginOverlap(Box)
  (params (OverlappedComponent :type Primitive%20Component%20Object%20Reference) (OtherActor :type Actor%20Object%20Reference) (OtherComp :type Primitive%20Component%20Object%20Reference) (OtherBodyIndex :type Integer) (bFromSweep :type Boolean) (SweepResult :type Hit%20Result%20Structure%20%28by%20ref%29))
  (Networking|SwitchHasAuthority
    (:Authority
      (if (Actor|ActorHasTag OtherActor "Player")
        (bind _player (Class|BPIPlayerBase|GetPlayerRef(Message) OtherActor))
        (Class|BPIPlayerBase|CanClimb(Message) _player true self)
        (Development|PrintString "set climb true")))))

(event OnComponentEndOverlap(Box)
  (params (OverlappedComponent :type Primitive%20Component%20Object%20Reference) (OtherActor :type Actor%20Object%20Reference) (OtherComp :type Primitive%20Component%20Object%20Reference) (OtherBodyIndex :type Integer))
  (Networking|SwitchHasAuthority
    (:Authority
      (if (Actor|ActorHasTag OtherActor "Player")
        (bind _player (Class|BPIPlayerBase|GetPlayerRef(Message) OtherActor))
        (Class|BPIPlayerBase|CanClimb(Message) _player false)
        (Development|PrintString "set climb false")))))

(event OnComponentBeginOverlap(UpperBox)
  (params (OverlappedComponent :type Primitive%20Component%20Object%20Reference) (OtherActor :type Actor%20Object%20Reference) (OtherComp :type Primitive%20Component%20Object%20Reference) (OtherBodyIndex :type Integer) (bFromSweep :type Boolean) (SweepResult :type Hit%20Result%20Structure%20%28by%20ref%29))
  (Networking|SwitchHasAuthority
    (:Authority
      (if (Actor|ActorHasTag OtherActor "Player")
        (bind _player (Class|BPIPlayerBase|GetPlayerRef(Message) OtherActor))
        (Class|BPIPlayerBase|SetCanClimbUp(Message) _player false)))))

(event OnComponentEndOverlap(UpperBox)
  (params (OverlappedComponent :type Primitive%20Component%20Object%20Reference) (OtherActor :type Actor%20Object%20Reference) (OtherComp :type Primitive%20Component%20Object%20Reference) (OtherBodyIndex :type Integer))
  (Networking|SwitchHasAuthority
    (:Authority
      (if (Actor|ActorHasTag OtherActor "Player")
        (bind _player (Class|BPIPlayerBase|GetPlayerRef(Message) OtherActor))
        (Class|BPIPlayerBase|SetCanClimbUp(Message) _player true)))))

(event EventBeginPlay)

(event Collision|EventActorBeginOverlap
  (params (OtherActor :type Actor%20Object%20Reference)))

(event EventTick
  (params (DeltaSeconds :type Float%20%28single-precision%29)))

(fn ConstructionScript)