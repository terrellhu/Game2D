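; Networked Paper2D enemy character that damages overlapping players on a looping timer, chases whoever hurts it, and respawns after death.
; Hits pause movement and AI logic for the flipbook's length, then either start a repeating AI move toward the attacker or trigger death, fade-out and delayed respawn at a random navigable point.
; Server events set state, while RepNotifies apply flipbooks, materials, fade color and spawn location; death sound is multicast.
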(event OnComponentBeginOverlap(Sphere)
  (params (OverlappedComponent :type Primitive%20Component%20Object%20Reference) (OtherActor :type Actor%20Object%20Reference) (OtherComp :type Primitive%20Component%20Object%20Reference) (OtherBodyIndex :type Integer) (bFromSweep :type Boolean) (SweepResult :type Hit%20Result%20Structure%20%28by%20ref%29))
  (Networking|SwitchHasAuthority
    (:Authority
      (if (Actor|ActorHasTag OtherActor "Player")
        (CallFunction|StartApplyDamage true)))))

(event OnComponentEndOverlap(Sphere)
  (params (OverlappedComponent :type Primitive%20Component%20Object%20Reference) (OtherActor :type Actor%20Object%20Reference) (OtherComp :type Primitive%20Component%20Object%20Reference) (OtherBodyIndex :type Integer))
  (Networking|SwitchHasAuthority
    (:Authority
      (if (Actor|ActorHasTag OtherActor "Player")
        (CallFunction|StartApplyDamage false)))))

(event Custom|SRV_SetMovementState
  (params (MovementState :type E_MovementState%20Enum :default "NewEnumerator0"))
  (Variables|Default|SetMovementState MovementState))

(event Custom|SRV_StartApplyDamage
  (params (ApplyDamage :type Boolean))
  (if ApplyDamage
    (bind _returnvalue (Utilities|Time|SetTimerbyEvent (delegate Custom|ApplyDamage) 0.1 true))
    (Variables|Default|SetApplyDamageHandle _returnvalue)
    (else
      (bind _output_get (Variables|Default|SetApplyDamageHandle ""))
      (Utilities|Time|ClearandInvalidateTimerbyHandle _output_get))))

(event Custom|ApplyDamage
  (for _array_element (Collision|GetOverlappingActors "/Game/Blueprints/Player/BP_PlayerCharacter.BP_PlayerCharacter_C" :!class /Script/Engine.Actor)
    (bind _player (Class|BPIPlayerBase|GetPlayerRef(Message) _array_element))
    (if (not (Variables|/Game/Blueprints/Player/BP_PlayerCharacter.BP_PlayerCharacter_C|GetGodMode _player))
      (Game|Damage|ApplyDamage _player (.Damage (Utilities|Struct|BreakST_EnemyInfo (Variables|Default|GetEnemyInfo))) (Pawn|GetController) 0))))

(event Custom|SRV_Death
  (params (IsDead :type Boolean))
  (bind _output_get (Variables|Default|SetIs%20Dead IsDead))
  (if _output_get
    (CallFunction|MCDeath (Utilities|Struct|BreakST_EnemyInfo (Variables|Default|GetEnemyInfo)) (Transformation|GetActorLocation))))

(event Custom|SRV_Respawn
  (bind _returnvalue (Actor|GetActorOfClass "/Script/NavigationSystem.NavMeshBoundsVolume"))
  (Variables|Default|SetSpawnLocation (Math|Vector|MakeVector (.X (Math|Vector|BreakVector (.RandomLocation (AI|Navigation|GetRandomReachablePointinRadius (Transformation|GetActorLocation) (.X (Math|Vector|BreakVector (.BoxExtent (Collision|GetActorBounds _returnvalue false false)))) 0 0)))) (.Y (Math|Vector|BreakVector (Transformation|GetActorLocation))) (+ (.Z (Math|Vector|BreakVector (.RandomLocation (AI|Navigation|GetRandomReachablePointinRadius (Transformation|GetActorLocation) (.X (Math|Vector|BreakVector (.BoxExtent (Collision|GetActorBounds _returnvalue false false)))) 0 0)))) 5e+01))))

(event Custom|SRV_ActorFade
  (params (Fade :type Boolean))
  (bind _output_get (Variables|Default|SetFade Fade))
  (if _output_get
    (bind _alpha (Timeline|FadingActor PlayFromStart)
      (:Update
        (Variables|Default|SetActorFadeColor (Math|Color|Lerp(LinearColor) "(R=1.000000,G=1.000000,B=1.000000,A=1.000000)" "(R=1.000000,G=1.000000,B=1.000000,A=0.000000)" _alpha)))
      (:Finished
        (if (Variables|Default|GetFade)
          (CallFunction|Death false))))
    (else
      (Pawn|Components|CharacterMovement|SetMovementMode (Variables|Character|GetCharacterMovement) "MOVE_Walking" 0)
      (Timeline|FadingActor Reverse))))

(event Custom|MC_Death
  (params (EnemyDeathSFX :type Sound%20Base%20Object%20Reference) (Location :type Vector))
  (Audio|PlaySoundatLocation EnemyDeathSFX Location "0, 0, 0" 1.0 1.0 0.0 0 0 0 0))

(event Game|Damage|EventAnyDamage
  (params (Damage :type Float%20%28single-precision%29) (DamageType :type Damage%20Type%20Object%20Reference) (InstigatedBy :type Controller%20Object%20Reference) (DamageCauser :type Actor%20Object%20Reference))
  (bind _returnvalue (Transformation|GetActorLocation))
  (bind (_x _y _z) (Math|Vector|BreakVector _returnvalue))
  (Variables|Default|SetPlayerController InstigatedBy)
  (CallFunction|SetMovementState "NewEnumerator6")
  (Pawn|Components|CharacterMovement|SetMovementMode (Variables|Character|GetCharacterMovement) "MOVE_None" 0)
  (bind _structout (Utilities|Struct|SetmembersinST_EnemyInfo (Variables|Default|GetEnemyInfo) (Math|Float|Clamp(Float) (- (.Health (Utilities|Struct|BreakST_EnemyInfo (Variables|Default|GetEnemyInfo))) Damage) 0.0 (.Health (Utilities|Struct|BreakST_EnemyInfo (Variables|Default|GetEnemyInfo))))))
  (Variables|Default|SetEnemyInfo _structout)
  (Components|Movement|StopMovementImmediately (Variables|Character|GetCharacterMovement))
  (bind _aicontroller (Class|BPIAIController|GetAIControllerRef(Message) (Pawn|GetController)))
  (AI|Logic|StopLogic (Variables|/Script/AIModule.AIController|GetBrainComponent _aicontroller) "Hit")
  (Utilities|FlowControl|Delay (Class|PaperFlipbookComponent|GetFlipbookLength (Variables|Default|GetSprite)))
  (if (> (.Health (Utilities|Struct|BreakST_EnemyInfo (Variables|Default|GetEnemyInfo))) 0.0)
    (Pawn|Components|CharacterMovement|SetMovementMode (Variables|Character|GetCharacterMovement) "MOVE_Walking" 0)
    (CallFunction|SetMovementState "NewEnumerator1")
    (AI|AIMoveTo self (Transformation|GetActorLocation (Pawn|GetControlledPawn (Variables|Default|GetPlayerController))) (Pawn|GetControlledPawn (Variables|Default|GetPlayerController)) 5.0 false :!label _label
      (:OnSuccess
        (bind _player (Class|BPIPlayerBase|GetPlayerRef(Message) (Pawn|GetControlledPawn (Variables|Default|GetPlayerController))))
        (if (not (Variables|/Game/Blueprints/Player/BP_PlayerCharacter.BP_PlayerCharacter_C|GetIs%20Dead _player))
          (AI|AIMoveTo (AI|GetAIController self) (Math|Vector|MakeVector (+ (Math|Float|SelectFloat -125.0 125.0 (< (.X (Math|Vector|BreakVector (Transformation|GetActorLocation (Pawn|GetControlledPawn (Variables|Default|GetPlayerController))))) _x)) _x) _y _z) 0 -1.0 "Default" "Default" true true
            (:OnMoveFinished
              (goto _label)))
          (else
            (bind _aicontroller_2 (Class|BPIAIController|GetAIControllerRef(Message) (Pawn|GetController)))
            (AI|Logic|StartLogic (Variables|/Script/AIModule.AIController|GetBrainComponent _aicontroller_2))))))
    (else
      (CallFunction|Death true)
      (Variables|/Script/Engine.PrimitiveComponent|SetbGenerateOverlapEvents (Variables|Default|GetSphere) false)
      (Variables|/Script/Engine.PrimitiveComponent|SetbGenerateOverlapEvents (Variables|Default|GetHitSphere) false)
      (CallFunction|ActorFade true)
      (Utilities|FlowControl|Delay (Variables|Default|GetRespawnTime))
      (bind _structout_2 (Utilities|Struct|SetmembersinST_EnemyInfo (Variables|Default|GetEnemyInfo) (.MaxHealth (Utilities|Struct|BreakST_EnemyInfo (Variables|Default|GetEnemyInfo)))))
      (Variables|Default|SetEnemyInfo _structout_2)
      (CallFunction|Respawn)
      (CallFunction|ActorFade false)
      (bind _aicontroller_3 (Class|BPIAIController|GetAIControllerRef(Message) (Pawn|GetController)))
      (AI|Logic|StartLogic (Variables|/Script/AIModule.AIController|GetBrainComponent _aicontroller_3))
      (Variables|/Script/Engine.PrimitiveComponent|SetbGenerateOverlapEvents (Variables|Default|GetSphere) true)
      (Variables|/Script/Engine.PrimitiveComponent|SetbGenerateOverlapEvents (Variables|Default|GetHitSphere) true))))

(event EventStartApplyDamage
  (params (ApplyDamage :type Boolean))
  (CallFunction|SRVStartApplyDamage ApplyDamage))

(event EventDeath
  (params (IsDead :type Boolean))
  (CallFunction|SRVDeath IsDead))

(event EventSetMovementState
  (params (IsMoveing :type E_MovementState%20Enum :default "NewEnumerator0"))
  (CallFunction|SRVSetMovementState IsMoveing))

(event EventRespawn
  (CallFunction|SRVRespawn))

(event EventActorFade
  (params (Fade :type Boolean))
  (CallFunction|SRVActorFade Fade))

(fn ConstructionScript
  (|CallParentFunction))

(fn OnRepIsMoving
  (bind _sprite (Variables|Default|GetSprite))
  (bind _enemyinfo (Variables|Default|GetEnemyInfo))
  (bind (_idleanimation _moveanimation) (Utilities|Struct|BreakST_EnemyInfo _enemyinfo))
  (if (Variables|Default|GetIsMoving)
    (Sprite|SetFlipbook _sprite _moveanimation)
    (else
      (Sprite|SetFlipbook _sprite _idleanimation))))

(fn OnRepMovementState
  (bind _enemyinfo (Variables|Default|GetEnemyInfo))
  (bind (_idleanimation _moveanimation _hitanimation _deathanimation) (Utilities|Struct|BreakST_EnemyInfo _enemyinfo))
  (switch Utilities|FlowControl|Switch|SwitchonE_MovementState (Variables|Default|GetMovementState)
    (:NewEnumerator0
      (LocalVariables|Setfilpbook _idleanimation))
    (:NewEnumerator1
      (LocalVariables|Setfilpbook _moveanimation))
    (:NewEnumerator6
      (LocalVariables|Setfilpbook _hitanimation))
    (:NewEnumerator7
      (LocalVariables|Setfilpbook _deathanimation)))
  (Sprite|SetFlipbook (Variables|Default|GetSprite) (LocalVariables|Getfilpbook)))

(fn OnRepIsDead
  (if (Variables|Default|GetIs%20Dead)
    (CallFunction|SetMovementState "NewEnumerator7")
    (Rendering|Material|SetMaterial (Variables|Default|GetSprite) 0 "/Paper2D/TranslucentUnlitSpriteMaterial.TranslucentUnlitSpriteMaterial")
    (else
      (CallFunction|SetMovementState "NewEnumerator0")
      (Rendering|Material|SetMaterial (Variables|Default|GetSprite) 0 "/Paper2D/MaskedUnlitSpriteMaterial.MaskedUnlitSpriteMaterial"))))

(fn OnRepSpawnLocation
  (Transformation|SetActorLocation (Variables|Default|GetSpawnLocation) false false))

(fn OnRepActorFadeColor
  (Sprite|SetSpriteColor (Variables|Default|GetSprite) (Variables|Default|GetActorFadeColor)))

(fn GetEnemyRef
  (return self))