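; Player character for a networked 2D flipbook platformer that runs, jumps, climbs, melee-attacks and dies.
; Input calls server events that set replicated state, whose OnRep functions switch flipbooks, movement modes and position, while multicasts play sounds and effects.
; Attacks damage overlapping enemies; taking damage causes knockback, GodMode flicker and a health UI update.
; A separately spawned camera follows via timers and timeline lerp; death-sound and respawn-reset logic is unconnected.
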(event Custom|UpdatePlayerCameraPosition
  ;[1 1 1] 更新摄像机位置
  (bind _playercamera (Variables|PlayerCamera|GetPlayerCamera)
    (:then
      (bind _movementalpha (Timeline|TL_PlayerCameraPosition PlayFromStart)
        (:Update
          (Transformation|SetActorLocation (Variables|PlayerCamera|GetPlayerCamera) (Math|Vector|Lerp(Vector) (Transformation|GetActorLocation _playercamera) (Variables|PlayerProperties|GetCurrentPlayerLocation) _movementalpha) false false))))
    (:else)))

(event Custom|SRV_SetMovementState
  (params (MovementState :type E_MovementState%20Enum :default "NewEnumerator0"))
  ;[1 1 1] 走
  (Variables|PlayerMovement|SetMovementState MovementState))

(event Custom|ClimbInput
  (bind _zaxis (Variables|PlayerMovement|GetZAxis))
  ;[1 1 1] 爬
  (if (or (and (Variables|Climbing|GetCanClimbUp) (> _zaxis 0.0)) (< _zaxis 0.0))
    (Utilities|Time|ClearandInvalidateTimerbyHandle (Variables|Climbing|GetCheckClimbInputHandle))
    (CallFunction|SetIsClimbing true)))

(event Custom|SRV_AdjustClimbingLocation
  (bind _returnvalue (Transformation|GetActorLocation))
  ;[1 1 1] 爬
  (bind _climbing_object (Variables|Climbing|GetClimbing%20Object)
    (:then
      (Variables|Climbing|SetClimbingLocation (Math|Vector|MakeVector (.x (Transformation|GetActorLocation _climbing_object)) (.y _returnvalue) (.z _returnvalue))))
    (:else)))

(event Custom|SRV_SetCanClimbUp
  (params (CanClimbUp :type Boolean))
  ;[1 1 1] 爬
  (Variables|Climbing|SetCanClimbUp CanClimbUp))

(event Custom|SRV_PauseClimbFlipbook
  (params (IsPause :type Boolean))
  ;[1 1 1] 爬
  (Variables|Climbing|SetisPauseClimbFlipbook IsPause))

(event Custom|SRV_Attack
  (params (IsAttacking :type Boolean))
  (bind _overlappingactors (Collision|GetOverlappingActors "/Game/Blueprints/Enemy/BP_EnemyCharacter.BP_EnemyCharacter_C" :!class /Script/Engine.Actor))
  (bind _returnvalue (Transformation|GetActorLocation))
  (bind _playerinfo (Variables|PlayerProperties|GetPlayerInfo))
  (bind (_attackhitsfx _attacksfx) (Utilities|Struct|BreakST_PlayerInfo _playerinfo))
  (Variables|Default|SetIs%20Attacking IsAttacking)
  (if (> (Utilities|Array|Length _overlappingactors) 0)
    (CallFunction|MCAttack _attackhitsfx _returnvalue)
    (for _array_element _overlappingactors
      (Game|Damage|ApplyDamage _array_element (* (.BaseDamage (Utilities|Struct|BreakST_PlayerInfo (Variables|PlayerProperties|GetPlayerInfo))) (Variables|Default|GetDamageFactor)) (Pawn|GetController) 0 "/Script/Engine.DamageType"))
    (else
      (CallFunction|MCAttack _attacksfx _returnvalue)))
  (Utilities|FlowControl|Delay (Class|PaperFlipbookComponent|GetFlipbookLength (Variables|Default|GetSprite)))
  (Variables|Default|SetIs%20Attacking false))

(event Custom|MC_Attack
  (params (AttackSFX :type Sound%20Base%20Object%20Reference) (Location :type Vector))
  (Audio|PlaySoundatLocation AttackSFX Location "0, 0, 0" 1.0 1.0 0.0 0 0 0 0))

(event Custom|SRV_DamageVFX
  (params (Material :type Material%20Interface%20Object%20Reference) (Color :type Linear%20Color%20Structure))
  (CallFunction|MCDamageVFX Material Color))

(event Custom|MC_DamageVFX
  (params (Material :type Material%20Interface%20Object%20Reference) (Color :type Linear%20Color%20Structure))
  (bind _returnvalue (Utilities|Time|SetTimerbyEvent (delegate Custom|DamageVFXLoop) (/ (Variables|Default|GetGodModeTime) 8.0) true))
  (Variables|Default|SetDamageVFXHandle _returnvalue)
  (Utilities|Time|SetTimerbyEvent (delegate Custom|StopDamageVFX) (Variables|Default|GetGodModeTime) true))

(event Custom|DamageVFXLoop
  (bind _sprite (Variables|Default|GetSprite))
  (bind _sprite_2 (Variables|Default|GetSprite))
  (Rendering|Material|SetMaterial _sprite_2 0 (stale Custom|MC_DamageVFX Material))
  (Sprite|SetSpriteColor _sprite_2 (stale Custom|MC_DamageVFX Color))
  (Utilities|FlowControl|Delay (/ (Variables|Default|GetGodModeTime) 16.0))
  (Rendering|Material|SetMaterial _sprite 0 "/Paper2D/MaskedUnlitSpriteMaterial.MaskedUnlitSpriteMaterial")
  (Sprite|SetSpriteColor _sprite "(R=1.000000,G=1.000000,B=1.000000,A=1.000000)"))

(event Custom|StopDamageVFX
  (Utilities|Time|ClearandInvalidateTimerbyHandle (Variables|Default|GetDamageVFXHandle)))

(event Custom|mc_Jump
  (params (Sound :type Sound%20Base%20Object%20Reference) (Location :type Vector))
  ;[1 1 1] 跳
  (Audio|PlaySoundatLocation Sound Location "0, 0, 0" 1.0 1.0 0.0 0 0 0 0))

(event Custom|SRV_Death
  (params (IsDead :type Boolean))
  (bind _output_get (Variables|Default|SetIs%20Dead IsDead)))

(event Custom|SRV_DamageImpulse
  (params (Impulse :type Vector))
  (CallFunction|MCDamageImpulse Impulse))

(event Custom|MC_DamageImpulse
  (params (Impulse :type Vector))
  (Physics|AddImpulse (Variables|Character|GetCharacterMovement) Impulse true))

(event Custom|MC_Death
  (params (DeathSFX :type Sound%20Base%20Object%20Reference) (Location :type Vector))
  (Audio|PlaySoundatLocation DeathSFX Location "0, 0, 0" 1.0 1.0 0.0 0 0 0 0))

(event Custom|SRV_Jump
  (params (Sound :type Sound%20Base%20Object%20Reference) (Location :type Vector))
  ;[1 1 1] 跳
  (CallFunction|McJump Sound Location))

(event Custom|SRV_SetPlayerSpawnLocation
  (bind _gamemode (Class|BPIGameMode|GetGameModeRef(Message) (Game|GetGameMode)))
  (Variables|PlayerProperties|SetPlayer%20Spawn%20Location (Variables|/Game/Blueprints/BP_GameMode.BP_GameMode_C|GetPlayerSpawnLocation _gamemode)))

(event Custom|CL_PausePlayerCamera
  (params (Pause :type Boolean))
  (bind _getcurrentplayerlocationhandle (Variables|PlayerProperties|GetGetCurrentPlayerLocationHandle))
  ;[1 1 1] 更新摄像机位置
  (if Pause
    (Utilities|Time|PauseTimerbyHandle _getcurrentplayerlocationhandle)
    (else
      (Utilities|Time|UnpauseTimerbyHandle _getcurrentplayerlocationhandle))))

(event Custom|SRV_CanClimb
  (params (CanClimb :type Boolean) (ClimbingObject :type Paper%20Sprite%20Actor%20Object%20Reference))
  ;[1 1 1] 爬
  (Variables|Climbing|SetClimbing%20Object ClimbingObject)
  (bind _output_get (Variables|Climbing|SetCan%20Climb CanClimb))
  (if _output_get
    (bind _returnvalue (Utilities|Time|SetTimerbyEvent (delegate Custom|ClimbInput) 0.1 true))
    (Variables|Climbing|SetCheckClimbInputHandle _returnvalue)
    (elif (Variables|Climbing|GetIsClimbing)
      (Utilities|Time|ClearandInvalidateTimerbyHandle (Variables|Climbing|GetCheckClimbInputHandle))
      (CallFunction|SetIsClimbing false))))

(event Custom|SRV_SetZAxisValue
  (params (Value :type Float%20%28double-precision%29))
  ;[1 1 1] 爬
  (Variables|PlayerMovement|SetZAxis Value))

(event Custom|SRV_SetIsClimbing
  (params (IsClimbing :type Boolean))
  ;[1 1 1] 爬
  (Variables|Climbing|SetIsClimbing IsClimbing))

(event Custom|AdjustClimbingLocation
  ;[1 1 1] 爬
  (CallFunction|SRVAdjustClimbingLocation))

(event EventBeginPlay
  (CallFunction|SetPlayerSpawnLocation)
  (Utilities|FlowControl|Delay 0.1)
  (bind _returnvalue (Game|SpawnActorfromClass "/Game/Blueprints/BP_Camera.BP_Camera_C" (Math|Transform|MakeTransform (Transformation|GetActorLocation)) "AdjustIfPossibleButAlwaysSpawn" "MultiplyWithRoot" 0 0))
  (Variables|PlayerCamera|SetPlayerCamera _returnvalue)
  (bind _playercontroller (Class|BPIPlayerController|GetPlayerControllerRef(Message) (Pawn|GetController)))
  (Utilities|IsValid _playercontroller
    (:Is%20Valid
      (Game|Player|SetViewTargetwithBlend _playercontroller (Variables|PlayerCamera|GetPlayerCamera) 0.0 "VTBlend_Linear" 0.0 false)
      ;[1 1 1] 更新摄像机位置
      (bind _returnvalue_2 (Utilities|Time|SetTimerbyEvent (delegate Custom|UpdatePlayerCameraPosition) 0.05 true))
      (Variables|PlayerCamera|SetUpdatePlayerCameraPositionHandle _returnvalue_2)
      (bind _returnvalue_3 (Utilities|Time|SetTimerbyFunctionName 0 "GetCurrentPlayerLocation" 0.1 true))
      (Variables|PlayerProperties|SetGetCurrentPlayerLocationHandle _returnvalue_3))))

(event Game|Damage|EventAnyDamage
  (params (Damage :type Float%20%28single-precision%29) (DamageType :type Damage%20Type%20Object%20Reference) (InstigatedBy :type Controller%20Object%20Reference) (DamageCauser :type Actor%20Object%20Reference))
  (Variables|Default|SetEnemyController InstigatedBy)
  (if (Variables|Climbing|GetIsClimbing)
    (Variables|Climbing|SetCan%20Climb false)
    (Variables|Climbing|SetIsClimbing false)
    (Variables|Climbing|SetisPauseClimbFlipbook false))
  (Variables|Default|SetGodMode true)
  (CallFunction|DamageImpulse (Math|Vector|MakeVector (Math|Float|SelectFloat -3e+02 3e+02 (< (.X (Math|Vector|BreakVector (Transformation|GetActorLocation))) (.X (Math|Vector|BreakVector (Transformation|GetActorLocation (Pawn|GetControlledPawn (Variables|Default|GetEnemyController))))))) 0.0 3e+02))
  (bind _structout (Utilities|Struct|SetmembersinST_PlayerInfo (Variables|PlayerProperties|GetPlayerInfo) (Math|Float|Clamp(Float) (- (.Health (Utilities|Struct|BreakST_PlayerInfo (Variables|PlayerProperties|GetPlayerInfo))) Damage) 0.0 (.Health (Utilities|Struct|BreakST_PlayerInfo (Variables|PlayerProperties|GetPlayerInfo))))))
  (bind _output_get (Variables|PlayerProperties|SetPlayerInfo _structout))
  (bind _playercontroller (Class|BPIPlayerController|GetPlayerControllerRef(Message) (Pawn|GetController)))
  (bind _enemy (Class|BPIEnemyBase|GetEnemyRef(Message) (Pawn|GetControlledPawn (Variables|Default|GetEnemyController))))
  (Class|BPIPlayerController|UpdateHealthValue(Message) _playercontroller (/ (.Health (Utilities|Struct|BreakST_PlayerInfo _output_get)) (.MaxHealth (Utilities|Struct|BreakST_PlayerInfo _output_get))) (.EnemyName (Utilities|Struct|BreakST_EnemyInfo (Variables|/Game/Blueprints/Enemy/BP_EnemyCharacter.BP_EnemyCharacter_C|GetEnemyInfo _enemy))))
  (if (== (.Health (Utilities|Struct|BreakST_PlayerInfo _output_get)) 0.0)
    (CallFunction|Death true)
    (else
      (CallFunction|DamageVFX "/Paper2D/TranslucentUnlitSpriteMaterial.TranslucentUnlitSpriteMaterial" "(R=1.000000,G=1.000000,B=1.000000,A=0.500000)")
      (Utilities|FlowControl|Delay (Variables|Default|GetGodModeTime))
      (Variables|Default|SetGodMode false))))

(event EventAttack
  (params (IsAttacking :type Boolean))
  (CallFunction|SRVAttack IsAttacking))

(event EventDeath
  (params (IsDead :type Boolean))
  (CallFunction|SRVDeath IsDead))

(event EventDamageImpulse
  (params (Impulse :type Vector :default "0, 0, 0"))
  (CallFunction|SRVDamageImpulse Impulse))

(event EventDamageVFX
  (params (PlayerMaterial :type Material%20Interface%20Object%20Reference) (PlayerColor :type Linear%20Color%20Structure))
  (CallFunction|SRVDamageVFX PlayerMaterial PlayerColor))

(event EventPausePlayerCamera
  (params (Pause :type Boolean))
  ;[1 1 1] 更新摄像机位置
  (CallFunction|CLPausePlayerCamera Pause))

(event EventSetMovementState
  (params (MovementState :type E_MovementState%20Enum :default "NewEnumerator0"))
  ;[1 1 1] 走
  (CallFunction|SRVSetMovementState MovementState))

(event EventSetPlayerSpawnLocation
  (CallFunction|SRVSetPlayerSpawnLocation))

(event EventCanClimb
  (params (CanClimb :type Boolean) (ClimbingObject :type Paper%20Sprite%20Actor%20Object%20Reference))
  ;[1 1 1] 爬
  (CallFunction|SRVCanClimb CanClimb ClimbingObject))

(event EventSetZAxisValue
  (params (Value :type Float%20%28double-precision%29))
  ;[1 1 1] 爬
  (CallFunction|SRVSetZAxisValue Value))

(event EventSetIsClimbing
  (params (IsClimbing :type Boolean))
  ;[1 1 1] 爬
  (CallFunction|SRVSetIsClimbing IsClimbing))

(event EventSetCanClimbUp
  (params (CanClimbUp :type Boolean))
  ;[1 1 1] 爬
  (CallFunction|SRVSetCanClimbUp CanClimbUp))

(event EventPauseClimbFlipbook
  (params (IsPause :type Boolean))
  ;[1 1 1] 爬
  (CallFunction|SRVPauseClimbFlipbook IsPause))

(event Input|ActionEvents|InputActionJump
  (params (Key :type Key%20Structure :default "None"))
  ;[1 1 1] 跳
  (:Pressed
    (if (not (Math|Boolean|ANDBoolean (not (Variables|Climbing|GetIsClimbing)) (AI|Components|NavMovement|IsFalling (Variables|Character|GetCharacterMovement)) (not (Variables|Default|GetIs%20Dead))))
      (Character|Jump)
      (CallFunction|SRVJump (.JumpSFX (Utilities|Struct|BreakST_PlayerInfo (Variables|PlayerProperties|GetPlayerInfo))) (Transformation|GetActorLocation)))))

(event Input|ActionEvents|InputActionAttack
  (params (Key :type Key%20Structure :default "None"))
  (:Pressed
    (if (and (not (Variables|Default|GetIs%20Attacking)) (not (Variables|Default|GetIs%20Dead)))
      (CallFunction|Attack true))))

(event Input|AxisEvents|InputAxisMoveRight/Left
  (params (AxisValue :type Float%20%28single-precision%29))
  ;[1 1 1] 走
  (if (Math|Boolean|ANDBoolean (not (Variables|Climbing|GetIsClimbing)) (not (Variables|Default|GetIs%20Attacking)) (not (Variables|Default|GetIs%20Dead)))
    (Pawn|Input|AddMovementInput (Math|Vector|GetForwardVector (Pawn|GetControlRotation :!class /Script/Engine.Pawn)) (* AxisValue (Variables|PlayerMovement|GetSpeedRate)) false)
    (if (AI|Components|NavMovement|IsFalling (Variables|Character|GetCharacterMovement))
      (if (> (.Z (Class|KismetMathLibrary|BreakVector3f (Transformation|GetVelocity))) 0.0)
        (CallFunction|SetMovementState "NewEnumerator3")
        (else
          (CallFunction|SetMovementState "NewEnumerator4")))
      (elif (== AxisValue 0.0)
        (CallFunction|SetMovementState "NewEnumerator0")
        (CallFunction|SetMovementState "NewEnumerator0")
        (elif (> AxisValue 0.0)
          (CallFunction|SetMovementState "NewEnumerator1")
          (else
            (CallFunction|SetMovementState "NewEnumerator2")))))))

(event Input|AxisEvents|InputAxisMoveUp/Down
  (params (AxisValue :type Float%20%28single-precision%29))
  ;[1 1 1] 爬
  (if (and (Variables|Climbing|GetCan%20Climb) (not (Variables|Default|GetIs%20Dead)))
    (CallFunction|SetZAxisValue AxisValue)
    (Pawn|Input|AddMovementInput (Math|Vector|GetUpVector (Pawn|GetControlRotation :!class /Script/Engine.Pawn)) AxisValue false)
    (if (Variables|Climbing|GetIsClimbing)
      (if (and (!= (Variables|PlayerMovement|GetZAxis) 0.0) (not (Audio|Components|Audio|IsPlaying (Variables|Default|GetSprite))))
        (CallFunction|PauseClimbFlipbook false)
        (elif (and (== (Variables|PlayerMovement|GetZAxis) 0.0) (Audio|Components|Audio|IsPlaying (Variables|Default|GetSprite)))
          (CallFunction|PauseClimbFlipbook true)
          (else
            (bind _climbing_object (Variables|Climbing|GetClimbing%20Object)
              (:then
                (if (!= (.x (Transformation|GetActorLocation _climbing_object)) (.x (Transformation|GetActorLocation)))
                  (CallFunction|AdjustClimbingLocation)))
              (:else))))))))

(fn ConstructionScript
  (|CallParentFunction))

(fn OnRepMovementState
  (bind _playerinfo (Variables|PlayerProperties|GetPlayerInfo))
  (bind _playerinfo_2 (Variables|PlayerProperties|GetPlayerInfo))
  (bind _sprite (Variables|Default|GetSprite))
  (bind _sprite_2 (Variables|Default|GetSprite))
  (bind (_jumpanim _attackanim _deathanim _fallanim) (Utilities|Struct|BreakST_PlayerInfo _playerinfo))
  (bind (_idleanim _runanim) (Utilities|Struct|BreakST_PlayerInfo _playerinfo_2))
  (if (not (Variables|Climbing|GetIsClimbing))
    (switch Utilities|FlowControl|Switch|SwitchonE_MovementState (Variables|PlayerMovement|GetMovementState)
      (:NewEnumerator0
        (Sprite|SetFlipbook (Variables|Default|GetSprite) _idleanim))
      (:NewEnumerator1
        (Transformation|SetRelativeRotation _sprite "0, 0, 0" false false)
        (Sprite|SetFlipbook _sprite _runanim))
      (:NewEnumerator2
        (Transformation|SetRelativeRotation _sprite_2 "0.000000,180.000000,0.000000" false false)
        (Sprite|SetFlipbook _sprite_2 _runanim))
      (:NewEnumerator3
        (Sprite|SetFlipbook (Variables|Default|GetSprite) _jumpanim))
      (:NewEnumerator4
        (Sprite|SetFlipbook (Variables|Default|GetSprite) _fallanim))
      (:NewEnumerator5
        (Sprite|SetFlipbook (Variables|Default|GetSprite) _attackanim))
      (:NewEnumerator7
        (Sprite|SetFlipbook (Variables|Default|GetSprite) _deathanim)))))

(fn OnRepPlayerSpawnLocation
  (Transformation|SetActorLocation (Variables|PlayerProperties|GetPlayer%20Spawn%20Location) false false))

(fn GetCurrentPlayerLocation
  (Variables|PlayerProperties|SetCurrentPlayerLocation (Transformation|GetActorLocation)))

(fn OnRepIsClimbing
  (bind _charactermovement (Variables|Character|GetCharacterMovement))
  (bind _sprite (Variables|Default|GetSprite))
  (bind _playerinfo (Variables|PlayerProperties|GetPlayerInfo))
  (bind _capsulecomponent (Variables|Default|GetCapsuleComponent))
  (bind (_attackanim _deathanim _fallanim _ropeanim) (Utilities|Struct|BreakST_PlayerInfo _playerinfo))
  (if (Variables|Climbing|GetIsClimbing)
    (Pawn|Components|CharacterMovement|SetMovementMode _charactermovement "MOVE_Flying" 0)
    (Collision|SetCollisionObjectType _capsulecomponent "ECC_GameTraceChannel1")
    (bind _asbp_climbing_actor_base (Utilities|Casting|CastToBP_ClimbingActorBase (Variables|Climbing|GetClimbing%20Object)))
    (switch Utilities|FlowControl|Switch|SwitchonE_ClimbingObjectType (Variables|/Game/Blueprints/Climbing/BP_ClimbingActorBase.BP_ClimbingActorBase_C|GetClimbingObjectType _asbp_climbing_actor_base)
      (:NewEnumerator0
        (Sprite|SetFlipbook _sprite _ropeanim)))
    (elif (not (Variables|Default|GetIs%20Dead))
      (Pawn|Components|CharacterMovement|SetMovementMode _charactermovement "MOVE_Falling" 0)
      (Collision|SetCollisionObjectType _capsulecomponent "ECC_Pawn")
      (Sprite|SetFlipbook _sprite _fallanim)
      (else
        (Pawn|Components|CharacterMovement|SetMovementMode _charactermovement "MOVE_Walking" 0)
        (Collision|SetCollisionObjectType _capsulecomponent "ECC_Pawn")
        (CallFunction|SetMovementState "NewEnumerator7")))))

(fn OnRepClimbingLocation
  (Transformation|SetActorLocation (Variables|Climbing|GetClimbingLocation) false false))

(fn OnRepIsPauseClimbFlipbook
  (bind _sprite (Variables|Default|GetSprite))
  (if (Variables|Climbing|GetisPauseClimbFlipbook)
    (Audio|Components|Audio|Stop _sprite)
    (else
      (Audio|Components|Audio|Play _sprite))))

(fn OnRepIsAttacking
  (if (Variables|Default|GetIs%20Attacking)
    (CallFunction|SetMovementState "NewEnumerator5")
    (elif (Variables|Default|GetIs%20Dead)
      (CallFunction|SetMovementState "NewEnumerator7")
      (else
        (CallFunction|SetMovementState "NewEnumerator0")))))

(fn OnRepIsDead
  (if (Variables|Default|GetIs%20Dead)
    (Components|Movement|StopMovementImmediately (Variables|Character|GetCharacterMovement))
    (CallFunction|SetMovementState "NewEnumerator7")))

(fn GetPlayerRef
  (return self))